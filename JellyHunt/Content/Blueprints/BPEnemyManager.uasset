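; Enemy manager actor that populates the surrounding navmesh with enemies, tracked as jellies, until a lifetime cap of fifty spawn attempts is reached.
; Tick calls SpawnEnemy every frame, which picks a random navigable point within a large radius of the manager and increments the counter.
; A random bool chooses between spawning MyNPC and a second spawn node that shows no class, and the counter counts both branches.
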(event EventBeginPlay)

(event Collision|EventActorBeginOverlap
  (params (OtherActor :type Actor%20Object%20Reference)))

(event EventTick
  (params (DeltaSeconds :type Float%20%28single-precision%29))
  (CallFunction|SpawnEnemy))

(fn ConstructionScript)

(fn SpawnEnemy
  (bind _self self)
  (bind _returnvalue (Transformation|GetActorLocation _self))
  (bind _randomlocation (Class|NavigationSystemV1|GetRandomPointinNavigableRadius _returnvalue 1e+04 0 "/Script/AIModule.NavFilter_AIControllerDefault"))
  (if (< (Variables|Default|GetJellyies%20Spawned) 5e+01)
    (if (Math|Random|RandomBool)
      (Game|SpawnActorfromClass "/Game/AI/MyNPC.MyNPC_C" (Math|Transform|MakeTransform _randomlocation "0, 0, 0" "1,1,1") "Undefined" 0 0)
      (else
        (Game|SpawnActorfromClass "/Game/AI/AngryNPC.AngryNPC_C" (Math|Transform|MakeTransform _randomlocation "0, 0, 0" "1,1,1") "Undefined" 0 0)))
    (Variables|Default|SetJellyies%20Spawned (+ (Variables|Default|GetJellyies%20Spawned) 1.0))))