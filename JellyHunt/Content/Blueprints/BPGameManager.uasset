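; BPGameManager is an actor that carries the Coins, Jelly and JellyFish counts to and from the game instance.
; BeginPlay casts the game instance to SaveGameWInstance, copies the three values into local variables and prints the coin count on screen.
; EndPlay writes Coins and Jelly back to that instance.
; The JellyFish write sits on the failed-cast branch, so it is not saved when the cast succeeds.
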(event EventBeginPlay
  (bind _assave_game_winstance (Utilities|Casting|CastToSaveGameWInstance (Game|GetGameInstance)))
  (Utilities|FlowControl|Sequence
    (:then_0
      (bind _output_get (Variables|Default|SetICoin (Variables|/Game/Blueprints/SaveGameWInstance.SaveGameWInstance_C|GetCoins _assave_game_winstance)))
      (Development|PrintString (Utilities|String|ToString(Integer) _output_get) true true "(R=1.000000,G=0.021375,B=0.000000,A=1.000000)"))
    (:then_1
      (Variables|Default|SetIJelly (Variables|/Game/Blueprints/SaveGameWInstance.SaveGameWInstance_C|GetJelly _assave_game_winstance)))
    (:then_2
      (Variables|Default|SetIJellyFish (Variables|/Game/Blueprints/SaveGameWInstance.SaveGameWInstance_C|GetJellyFish _assave_game_winstance)))))

(event EventEndPlay
  (params (EndPlayReason :type EEndPlayReason%20Enum :default "Destroyed"))
  (bind _assave_game_winstance (Utilities|Casting|CastToSaveGameWInstance (Game|GetGameInstance))
    (:then
      (Utilities|FlowControl|Sequence
        (:then_0
          (Variables|/Game/Blueprints/SaveGameWInstance.SaveGameWInstance_C|SetCoins _assave_game_winstance (Variables|Default|GetICoin)))
        (:then_1
          (Variables|/Game/Blueprints/SaveGameWInstance.SaveGameWInstance_C|SetJelly _assave_game_winstance (Variables|Default|GetIJelly)))))
    (:CastFailed
      (Variables|/Game/Blueprints/SaveGameWInstance.SaveGameWInstance_C|SetJellyFish _assave_game_winstance (Variables|Default|GetIJellyFish)))))

(event Collision|EventActorBeginOverlap
  (params (OtherActor :type Actor%20Object%20Reference)))

(fn ConstructionScript)