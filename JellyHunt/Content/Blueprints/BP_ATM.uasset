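; BP_ATM is an interactable machine that converts the player's coins into jelly at 20 coins per jelly.
; A box overlap toggles a flag, and Tick polls for the E key while it is set, checking the Player tag.
; Conversion updates the first BPGameManager found, adding the integer quotient to jelly and keeping the remainder as coins, with debug prints along the way.
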(event OnComponentBeginOverlap(Box)
  (params (OverlappedComponent :type Primitive%20Component%20Object%20Reference) (OtherActor :type Actor%20Object%20Reference) (OtherComp :type Primitive%20Component%20Object%20Reference) (OtherBodyIndex :type Integer) (bFromSweep :type Boolean) (SweepResult :type Hit%20Result%20Structure%20%28by%20ref%29))
  (Variables|Default|SetcollidesWithPlayer true)
  (Development|PrintString "colHello"))

(event OnComponentEndOverlap(Box)
  (params (OverlappedComponent :type Primitive%20Component%20Object%20Reference) (OtherActor :type Actor%20Object%20Reference) (OtherComp :type Primitive%20Component%20Object%20Reference) (OtherBodyIndex :type Integer))
  (Variables|Default|SetcollidesWithPlayer false)
  (Development|PrintString "nooocolHello"))

(event EventBeginPlay
  (|CallParentFunction)
  (Variables|Default|SetInteractionText "Press [E] to convert coins to jelly"))

(event Collision|EventActorBeginOverlap
  (params (OtherActor :type Actor%20Object%20Reference))
  (|CallParentFunction OtherActor))

(event EventTick
  (params (DeltaSeconds :type Float%20%28single-precision%29))
  (|CallParentFunction DeltaSeconds)
  (if (Variables|Default|GetcollidesWithPlayer)
    (Development|PrintString "Hello")
    (if (Actor|ActorHasTag (stale OnComponentBeginOverlap(Box) OtherActor) "Player")
      (if (Game|Player|WasInputKeyJustPressed (Game|GetPlayerController 0) "E")
        (Development|PrintString "E pressed")
        (bind _outactors (Actor|GetAllActorsOfClass "/Game/Blueprints/BPGameManager.BPGameManager_C"))
        (Development|PrintString "convert jelly")
        (if (>= (/ (Variables|/Game/Blueprints/BPGameManager.BPGameManager_C|GetICoin (Utilities|Array|Get(acopy) _outactors)) 20) 0)
          (Utilities|FlowControl|Sequence
            (:then_0
              (Variables|/Game/Blueprints/BPGameManager.BPGameManager_C|SetIJelly (Utilities|Array|Get(acopy) _outactors) (+ (Variables|/Game/Blueprints/BPGameManager.BPGameManager_C|GetIJelly (Utilities|Array|Get(acopy) _outactors)) (/ (Variables|/Game/Blueprints/BPGameManager.BPGameManager_C|GetICoin (Utilities|Array|Get(acopy) _outactors)) 20))))
            (:then_1
              (Variables|/Game/Blueprints/BPGameManager.BPGameManager_C|SetICoin (Utilities|Array|Get(acopy) _outactors) (Math|Integer|%(Integer) (Variables|/Game/Blueprints/BPGameManager.BPGameManager_C|GetICoin (Utilities|Array|Get(acopy) _outactors)) 20)))))))))

(fn ConstructionScript
  (|CallParentFunction))