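; BP_DoorToJellyFields is an interactable door that takes the player to the JellyGrounds level, shown by a "Press [E] To Jellyfish Fields" prompt.
; On BeginPlay it sets the interaction text and caches the player's FirstPersonCharacter.
; Its Use override saves the game to that character's save slot, opens the level with the slot name passed as the options string, then calls the parent Use.
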(event EventBeginPlay
  (|CallParentFunction)
  (Variables|Default|SetInteractionText "Press [E] To Jellyfish Fields")
  (bind _asfirst_person_character (Utilities|Casting|CastToFirstPersonCharacter (Game|GetPlayerCharacter 0)))
  (Variables|Default|SetCharacterReference _asfirst_person_character))

(event Collision|EventActorBeginOverlap
  (params (OtherActor :type Actor%20Object%20Reference))
  (|CallParentFunction OtherActor) ; This node is disabled and will not be called.\nDrag off pins to build functionality.
)

(event EventTick
  (params (DeltaSeconds :type Float%20%28single-precision%29))
  (|CallParentFunction DeltaSeconds) ; This node is disabled and will not be called.\nDrag off pins to build functionality.
)

(fn ConstructionScript
  (|CallParentFunction))

(fn Use
  (bind _characterreference (Variables|Default|GetCharacterReference))
  (bind _saveslotname (Variables|/Game/FirstPersonBP/Blueprints/FirstPersonCharacter.FirstPersonCharacter_C|GetSaveSlotName _characterreference))
  (Default|SaveGame _characterreference _saveslotname)
  (Game|OpenLevel(byName) "JellyGrounds" false _saveslotname)
  (|CallParentFunction))