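; BP_JellyConverter is an actor that converts the player's jellyfish into jelly at four to one.
; BeginPlay sets an interaction prompt, then runs the conversion immediately on the first BPGameManager found, with no interaction event in this Blueprint.
; The jelly count is overwritten with the quotient rather than added to, and the remainder stays as jellyfish.
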(event EventBeginPlay
  (|CallParentFunction)
  (Variables|Default|SetInteractionText "Press [E] to convert Jellyfish Into Jelly")
  (bind _outactors (Actor|GetAllActorsOfClass "/Game/Blueprints/BPGameManager.BPGameManager_C"))
  (Development|PrintString "convert jelly")
  (if (>= (/ (Variables|/Game/Blueprints/BPGameManager.BPGameManager_C|GetIJellyFish (Utilities|Array|Get(acopy) _outactors)) 4) 0)
    (Utilities|FlowControl|Sequence
      (:then_0
        (Variables|/Game/Blueprints/BPGameManager.BPGameManager_C|SetIJelly (Utilities|Array|Get(acopy) _outactors) (/ (Variables|/Game/Blueprints/BPGameManager.BPGameManager_C|GetIJellyFish (Utilities|Array|Get(acopy) _outactors)) 4)))
      (:then_1
        (Variables|/Game/Blueprints/BPGameManager.BPGameManager_C|SetIJellyFish (Utilities|Array|Get(acopy) _outactors) (Math|Integer|%(Integer) (Variables|/Game/Blueprints/BPGameManager.BPGameManager_C|GetIJellyFish (Utilities|Array|Get(acopy) _outactors)) 4))))))

(event Collision|EventActorBeginOverlap
  (params (OtherActor :type Actor%20Object%20Reference))
  (|CallParentFunction OtherActor) ; This node is disabled and will not be called.\nDrag off pins to build functionality.
)

(event EventTick
  (params (DeltaSeconds :type Float%20%28single-precision%29))
  (|CallParentFunction DeltaSeconds))

(fn ConstructionScript
  (|CallParentFunction))